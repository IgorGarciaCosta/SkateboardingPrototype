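; Music controller that plays random songs from a list as 2D sound, starting on BeginPlay and continuing indefinitely.
; Each pick rerolls until it differs from the current song, so a single-entry list would loop endlessly.
; A timer fires one fade length before the track ends, fading it out before the next spawns.
; PauseMusic and ResumeMusic pause and resume both audio and timer together.
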(event Custom|ChangeSong
  (bind _fadedout_ (CallFunction|TrytoFadeOutOldSong))
  (if _fadedout_
    (Utilities|FlowControl|Delay (Variables|Default|GetFadeDurantion)))
  (Variables|Default|SetCurrentSoundSoundBase (CallFunction|SelectNewSOng))
  (bind _returnvalue (Audio|SpawnSound2D (Variables|Default|GetCurrentSoundSoundBase) (Variables|Default|GetVolume%20Multiplier) 1.0 0.0 0))
  (Variables|Default|SetCurrentSongRef _returnvalue)
  (bind _returnvalue_2 (Utilities|Time|SetTimerbyEvent (delegate Custom|CallChangeSong) (- (Variables|/Script/Engine.SoundBase|GetDuration (Variables|Default|GetCurrentSoundSoundBase)) (Variables|Default|GetFadeDurantion))))
  (Variables|Default|SetCurrentMusicTimerHandle _returnvalue_2))

(event Custom|CallChangeSong
  (CallFunction|ChangeSong))

(event EventBeginPlay
  (CallFunction|ChangeSong))

(event Collision|EventActorBeginOverlap
  (params (OtherActor :type Actor%20Object%20Reference)))

(event EventTick
  (params (DeltaSeconds :type Float%20%28single-precision%29)))

(fn ConstructionScript)

(fn SelectNewSOng
  (bind _songs (Variables|Default|GetSongs))
  (LocalVariables|SetProvisionalSong (Utilities|Array|Get(acopy) _songs (Math|Random|RandomIntegerinRange 0 (Utilities|Array|LastIndex _songs))) :!label _label)
  (if (== (Variables|Default|GetCurrentSoundSoundBase) (LocalVariables|GetProvisionalSong))
    (goto _label)
    (else
      (return (LocalVariables|GetProvisionalSong)))))

(fn TrytoFadeOutOldSong
  (bind _currentsongref (Variables|Default|GetCurrentSongRef))
  (Utilities|IsValid _currentsongref
    (:Is%20Valid
      (Audio|Components|Audio|FadeOut _currentsongref (Variables|Default|GetFadeDurantion) 0.0 "Linear" :!class /Script/Engine.AudioComponent)
      (return true))
    (:Is%20Not%20Valid
      (return false))))

(fn PauseMusic
  (Utilities|Time|PauseTimerbyHandle (Variables|Default|GetCurrentMusicTimerHandle))
  (Class|AudioComponent|SetPaused (Variables|Default|GetCurrentSongRef) true))

(fn ResumeMusic
  (Utilities|Time|UnpauseTimerbyHandle (Variables|Default|GetCurrentMusicTimerHandle))
  (Class|AudioComponent|SetPaused (Variables|Default|GetCurrentSongRef) false))